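; Base enemy actor for an Octopath-style game that starts combat when a BP_Therion overlaps it.
; On overlap it toggles the player's combat state and jumps back along a timeline-driven arc, then hands both combatants to the GameMode.
; Attacks chain that jump with delayed moves toward the player and back.
; Non-negative damage flashes the sprite material and lerps HP down, or fades opacity and destroys the actor at zero.
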(event Custom|doDeadAnimation
  (bind _opacity (Timeline|Cronograma Play)
    (:Update
      (Rendering|Material|SetScalarParameterValue (Variables|Default|GetMaterialInstance) "Opacity" _opacity :!class /Script/Engine.MaterialInstanceDynamic))
    (:Finished
      (Actor|DestroyActor))))

(event Custom|TriggerEnemyFlash
  (params (Multiplier :type Float%20%28single-precision%29) (Color :type Linear%20Color%20Structure) (PlayRate :type Float%20%28single-precision%29))
  ;[1 1 1] Sprite Flash
  (Rendering|Material|SetScalarParameterValue (Variables|Default|GetMaterialInstance) "FlashMultiplier" Multiplier :!class /Script/Engine.MaterialInstanceDynamic)
  (Rendering|Material|SetVectorParameterValue (Variables|Default|GetMaterialInstance) "FlashColor" Color :!class /Script/Engine.MaterialInstanceDynamic)
  (Components|Timeline|SetPlayRate (Variables|Default|GetFlash%20Multiplier) PlayRate)
  (bind _alpha (Timeline|Flash%20Multiplier PlayFromStart)
    (:Update
      (Rendering|Material|SetScalarParameterValue (Variables|Default|GetMaterialInstance) "FlashMultiplier" (Math|Float|Lerp 0.0 Multiplier _alpha) :!class /Script/Engine.MaterialInstanceDynamic))))

(event Custom|getDamage
  (params (Damage :type Float%20%28double-precision%29))
  (bind _returnvalue (>= Damage 0.0))
  ;[1 1 1] Heal check
  (if _returnvalue ; No puedes esquivar heals
    ;[1 1 1] Flash animation
    (CallFunction|TriggerEnemyFlash 0.05 (select _returnvalue "(R=1.000000,G=0.046538,B=0.000000,A=1.000000)" "(R=0.000000,G=1.000000,B=0.106025,A=1.000000)") 5.0))
  ;[1 1 1] Damage animation (if not heal)
  (if _returnvalue
    ;[1 1 1] Gestión vida
    (bind _output_get (Variables|Default|SetTargetHP (Math|Float|Min(Float) (Math|Float|Max(Float) (- (Variables|Default|GetCurrentHP) Damage) 0.0) (Variables|Default|GetMaxHP))))
    (if (> _output_get 0.0)
      ;[1 1 1] Lerp vida
      (bind _alpha (Timeline|Cronograma_0 PlayFromStart)
        (:Update
          (Variables|Default|SetCurrentHP (Math|Float|Lerp (Variables|Default|GetCurrentHP) (Variables|Default|GetTargetHP) _alpha))))
      (else
        ;[1 1 1] Gestión derrota
        (CallFunction|DoDeadAnimation)
        (Timeline|Cronograma_0 PlayFromStart)))))

(event Custom|doJump
  (params (Player :type BP%20Therion%20Object%20Reference))
  ;[1 1 1] doJump
  (bind (_direction _arcy _arcx) (Timeline|Cronograma_2 PlayFromStart)
    (:Update
      (Transformation|SetActorLocation (+ (Math|Vector|Lerp(Vector) (Variables|Default|GetStartJump) (Variables|Default|GetEndJump) _arcx) (Math|Vector|MakeVector 0.0 0.0 (* _arcy (Variables|Default|GetJumpHeight)))) false false))
    (:Finished
      (if (Variables|Default|Getcolision)
        (Variables|Default|SetStartAttack (Transformation|GetActorLocation))
        (else
          (Variables|Default|Setcolision true)
          (Default|StartCombat (Variables|Default|GetGameMode) Player self))))))

(event Custom|doAttack
  (params (Player :type BP%20Therion%20Object%20Reference))
  (bind _returnvalue (Transformation|GetActorLocation))
  (bind (_x _y _z) (Math|Vector|BreakVector _returnvalue))
  (Variables|Default|SetStartJump _returnvalue)
  (Variables|Default|SetEndJump (Math|Vector|MakeVector (- (.X (Math|Vector|BreakVector (Transformation|GetActorLocation Player))) 3e+02) _y _z))
  (CallFunction|DoJump)
  (Utilities|FlowControl|Delay 1.0)
  (Components|MoveComponentTo 0 (+ (Variables|Default|GetStartJump) (* (Math|Vector|GetForwardVector "0, 0, 0") "100.000000,0.000000,0.000000")) "0, 0, 0" false false 0.2 false)
  (Utilities|FlowControl|Delay 1.0)
  (Components|MoveComponentTo 0 (Variables|Default|GetStartAttack) "0, 0, 0" false false 0.2 false)
  (Variables|Default|SetEndJump (Variables|Default|GetStartJump))
  (Variables|Default|SetStartJump (Transformation|GetActorLocation))
  (CallFunction|DoJump))

(event EventBeginPlay
  (bind _asgm_octopath_game_mode (Utilities|Casting|CastToGM_OctopathGameMode (Game|GetGameMode)))
  (Variables|Default|SetGameMode _asgm_octopath_game_mode))

(event Collision|EventActorBeginOverlap
  (params (OtherActor :type Actor%20Object%20Reference))
  ;[1 1 1] Start Combat
  (bind _asbp_therion (Utilities|Casting|CastToBP_Therion OtherActor))
  (Variables|Default|SetcombatSpeed (Math|Random|RandomFloat))
  (Default|ToggleinCombat _asbp_therion)
  (Variables|Default|SetStartJump (Transformation|GetActorLocation))
  (Variables|Default|SetEndJump (- (Transformation|GetActorLocation) "500.000000,0.000000,0.000000"))
  (CallFunction|DoJump _asbp_therion))

(event EventTick
  (params (DeltaSeconds :type Float%20%28single-precision%29)))

(fn ConstructionScript)

(fn StartCombat)