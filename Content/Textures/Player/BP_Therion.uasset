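; Therion player character: a flipbook-animated pawn with walk/run movement, combat animations and HP/MP.
; Tick picks idle, movement, defend or combat-idle flipbooks unless IsInAction holds a one-shot or repeated animation until OnFinishedPlaying.
; PlayerDamaged handles random dodges, halved damage when defending, and death; healing and MP restore reuse the damage and MP-use events with negated values.
; Timelines lerp HP/MP and drive colored flashes through a dynamic sprite material.
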(event OnFinishedPlaying(Sprite)
  (bind _sprite (Variables|Default|GetSprite))
  ;[1 1 1] When animation ends
  (if (not (Variables|Default|GetisDead))
    (if (Variables|Default|GetisRepeatingAnimation)
      (bind _output_get (Variables|Default|SetRepeatingAnimationCounter (- (Variables|Default|GetRepeatingAnimationCounter) 1)))
      (Sprite|SetFlipbook (Variables|Default|GetSprite) (Variables|Default|GetRepeatingFlipbook))
      (Components|Timeline|PlayfromStart (Variables|Default|GetSprite))
      (if (not (> _output_get 0))
        (Variables|Default|SetisRepeatingAnimation false)
        (Components|Timeline|SetLooping _sprite true :!label _label)
        (Components|Timeline|PlayfromStart _sprite)
        (Variables|Default|SetisInAction false))
      (else
        (goto _label)))))

(event Custom|UpdateAnimations
  (bind _charactermovement (Variables|Character|GetCharacterMovement))
  (bind _velocity (Variables|/Script/Engine.MovementComponent|GetVelocity _charactermovement))
  (bind (_x _y) (Math|Vector|BreakVector _velocity))
  (bind _returnvalue (Math|Float|InRange(Float) _x -5e+01 5e+01))
  (bind _returnvalue_2 (Math|Float|InRange(Float) _y -5e+01 5e+01))
  ;[1 1 1] WASD Movement Animations
  (if (not (Variables|Default|GetisInAction))
    (if (Variables|Default|GetisDefending)
      (Sprite|SetFlipbook (Variables|Default|GetSprite) "/Game/Textures/Player/Therion/All/FB_Defending.FB_Defending")
      (elif (Variables|Default|GetisInCombat)
        (Sprite|SetFlipbook (Variables|Default|GetSprite) "/Game/Textures/Player/Therion/All/FB_IdleCombat.FB_IdleCombat")
        (elif (and _returnvalue _returnvalue_2)
          (Sprite|SetFlipbook (Variables|Default|GetSprite) (Utilities|Select :Index (Variables|Default|GetFacingDirection) :NewEnumerator1 "/Game/Textures/Player/Therion/All/FB_Player_IdleUp.FB_Player_IdleUp" :NewEnumerator2 "/Game/Textures/Player/Therion/All/FB_Player_IdleDown.FB_Player_IdleDown" :NewEnumerator3 "/Game/Textures/Player/Therion/All/FB_Player_IdleLeft.FB_Player_IdleLeft" :NewEnumerator4 "/Game/Textures/Player/Therion/All/FB_Player_IdleRight.FB_Player_IdleRight"))
          (else
            (if _returnvalue_2
              _
              (else
                (Variables|Default|SetFacingDirection (select (> _y 0.0) "NewEnumerator2" "NewEnumerator1"))))
            (if _returnvalue
              _
              (else
                (Variables|Default|SetFacingDirection (select (> _x 0.0) "NewEnumerator4" "NewEnumerator3"))))
            (if (Variables|Default|GetisRunning)
              (Sprite|SetFlipbook (Variables|Default|GetSprite) (Utilities|Select :Index (Variables|Default|GetFacingDirection) :NewEnumerator1 "/Game/Textures/Player/Therion/All/FB_Player_RunUp.FB_Player_RunUp" :NewEnumerator2 "/Game/Textures/Player/Therion/All/FB_Player_RunDown.FB_Player_RunDown" :NewEnumerator3 "/Game/Textures/Player/Therion/All/FB_Player_RunLeft.FB_Player_RunLeft" :NewEnumerator4 "/Game/Textures/Player/Therion/All/FB_Player_RunRigh.FB_Player_RunRigh"))
              (else
                (Sprite|SetFlipbook (Variables|Default|GetSprite) (Utilities|Select :Index (Variables|Default|GetFacingDirection) :NewEnumerator1 "/Game/Textures/Player/Therion/All/FB_Player_WalkUp.FB_Player_WalkUp" :NewEnumerator2 "/Game/Textures/Player/Therion/All/FB_Player_WalkDown.FB_Player_WalkDown" :NewEnumerator3 "/Game/Textures/Player/Therion/All/FB_Player_WalkLeft.FB_Player_WalkLeft" :NewEnumerator4 "/Game/Textures/Player/Therion/All/FB_Player_WalkRight.FB_Player_WalkRight"))))))))))

(event Custom|doPunchAnimation
  (bind _sprite (Variables|Default|GetSprite))
  ;[1 1 1] Combat animations
  (if (not (Variables|Default|GetisInAction))
    (Variables|Default|SetisInAction true)
    (Components|Timeline|SetLooping _sprite false)
    (Sprite|SetFlipbook _sprite "/Game/Textures/Player/Therion/All/FB_PunchAttack.FB_PunchAttack")))

(event Custom|TriggerFlash
  (params (Multiplier :type Float%20%28single-precision%29) (Color :type Linear%20Color%20Structure) (PlayRate :type Float%20%28single-precision%29))
  ;[1 1 1] Player Sprite Flash
  (Rendering|Material|SetScalarParameterValue (Variables|Default|GetDynamicSpriteMaterial) "FlashMultiplier" Multiplier :!class /Script/Engine.MaterialInstanceDynamic)
  (Rendering|Material|SetVectorParameterValue (Variables|Default|GetDynamicSpriteMaterial) "FlashColor" Color :!class /Script/Engine.MaterialInstanceDynamic)
  (Components|Timeline|SetPlayRate (Variables|Default|GetFlashMultiplier) PlayRate)
  (bind _alpha (Timeline|FlashMultiplier PlayFromStart)
    (:Update
      (Rendering|Material|SetScalarParameterValue (Variables|Default|GetDynamicSpriteMaterial) "FlashMultiplier" (Math|Float|Lerp 0.0 Multiplier _alpha) :!class /Script/Engine.MaterialInstanceDynamic))))

(event Custom|PlayerDamaged
  (params (Damage :type Float%20%28double-precision%29))
  (bind _returnvalue (>= Damage 0.0))
  ;[1 1 1] HP system
  ;;[1 1 1] Heal check + iframe
  (if (not (Variables|Default|GetisInvulnerable))
    ;;[1 1 1] Gestión dodge
    (if _returnvalue ; No puedes esquivar heals
      (if (> (Math|Random|RandomIntegerinRange 1 100) (Variables|Default|GetDodgeRate))
        ;;[1 1 1] Flash animation
        (CallFunction|TriggerFlash 0.05 (select _returnvalue "(R=1.000000,G=0.046538,B=0.000000,A=1.000000)" "(R=0.000000,G=1.000000,B=0.106025,A=1.000000)") 3.0 :!label _label)
        ;;[1 1 1] Damage animation (if not heal)
        (if _returnvalue
          (CallFunction|DoDamagedAnimation))
        ;;[1 1 1] Gestión vida
        (bind _output_get (Variables|Default|SetTargetHP (Math|Float|Min(Float) (Math|Float|Max(Float) (- (Variables|Default|GetCurrentHP) (select (Variables|Default|GetisDefending) (/ Damage 2.0) Damage)) 0.0) (Variables|Default|GetMaxHP))))
        (if (> _output_get 0.0)
          ;;[1 1 1] Lerp vida
          (bind _alpha (Timeline|HealthLerpTimeline PlayFromStart)
            (:Update
              (Variables|Default|SetCurrentHP (Math|Float|Lerp (Variables|Default|GetCurrentHP) (Variables|Default|GetTargetHP) _alpha)))
            (:Finished
              (Variables|Default|SetisInvulnerable false)))
          (else
            ;;[1 1 1] Gestión game over
            (CallFunction|DoDeadAnimation)
            (Variables|Default|SetisDead true)
            (Timeline|HealthLerpTimeline PlayFromStart)))
        (else
          (CallFunction|DoDodgeAnimation)
          (CallFunction|TriggerFlash 0.01 "(R=0.000000,G=1.000000,B=0.909775,A=1.000000)" 2.0)))
      (else
        (goto _label)))))

(event Custom|PlayerUseMP
  (params (Mana :type Float%20%28double-precision%29))
  ;[1 1 1] MP system
  ;;[1 1 1] Flash animation
  (CallFunction|TriggerFlash 0.05 "(R=0.000000,G=0.027881,B=1.000000,A=1.000000)" 3.0)
  ;;[1 1 1] Gestión MP
  (Variables|Default|SetTargetMP (Math|Float|Min(Float) (Math|Float|Max(Float) (- (Variables|Default|GetCurrentMP) Mana) 0.0) (Variables|Default|GetMaxMP)))
  ;;[1 1 1] Lerp MP
  (bind _alpha (Timeline|MPLerpTimeline PlayFromStart)
    (:Update
      (Variables|Default|SetCurrentMP (Math|Float|Lerp (Variables|Default|GetCurrentMP) (Variables|Default|GetTargetMP) _alpha)))))

(event Custom|doDamagedAnimation
  (bind _sprite (Variables|Default|GetSprite))
  ;[1 1 1] Combat animations
  (if (not (Variables|Default|GetisInAction))
    (Variables|Default|SetisInAction true)
    (Components|Timeline|SetLooping _sprite false)
    (Sprite|SetFlipbook _sprite "/Game/Textures/Player/Therion/All/FB_Damaged.FB_Damaged")))

(event Custom|doThreePunchesAnimation
  ;[1 1 1] Combat animations
  (Variables|Default|SetRepeatingFlipbook "/Game/Textures/Player/Therion/All/FB_PunchAttack.FB_PunchAttack")
  (Variables|Default|SetisRepeatingAnimation true)
  (CallFunction|DoPunchAnimation)
  (Variables|Default|SetRepeatingAnimationCounter 3))

(event Custom|doWinAnimation
  (bind _sprite (Variables|Default|GetSprite))
  ;[1 1 1] Combat animations
  (if (not (Variables|Default|GetisInAction))
    (Variables|Default|SetisInAction true)
    (Components|Timeline|SetLooping _sprite false)
    (Sprite|SetFlipbook _sprite "/Game/Textures/Player/Therion/All/FB_Win.FB_Win")))

(event Custom|doDeadAnimation
  (bind _sprite (Variables|Default|GetSprite))
  ;[1 1 1] Combat animations
  (Variables|Default|SetisInAction true)
  (Components|Timeline|SetLooping _sprite false)
  (Sprite|SetFlipbook _sprite "/Game/Textures/Player/Therion/All/FB_Dead.FB_Dead"))

(event Custom|doDodgeAnimation
  (bind _sprite (Variables|Default|GetSprite))
  ;[1 1 1] Combat animations
  (if (not (Variables|Default|GetisInAction))
    (Variables|Default|SetisInAction true)
    (Components|Timeline|SetLooping _sprite false)
    (Sprite|SetFlipbook _sprite "/Game/Textures/Player/Therion/All/FB_Dodge.FB_Dodge")))

(event Custom|doStabAnimation
  (bind _sprite (Variables|Default|GetSprite))
  ;[1 1 1] Combat animations
  (if (not (Variables|Default|GetisInAction))
    (Variables|Default|SetisInAction true)
    (Components|Timeline|SetLooping _sprite false)
    (Sprite|SetFlipbook _sprite "/Game/Textures/Player/Therion/All/FB_Stab.FB_Stab")))

(event Input|EnhancedActionEvents|EnhancedInputActionIA_Move
  (params (ActionValue :type Vector%202D%20Structure) (ElapsedSeconds :type Float%20%28double-precision%29) (TriggeredSeconds :type Float%20%28double-precision%29) (InputAction :type Input%20Action%20Object%20Reference :default "/Game/Textures/Player/Input/IA_Move.IA_Move"))
  (bind _returnvalue (Pawn|GetControlRotation :!class /Script/Engine.Pawn))
  (bind _yaw (Math|Rotator|BreakRotator _returnvalue))
  (bind _returnvalue_2 (Math|Rotator|MakeRotator 0.0 0.0 _yaw))
  ;[1 1 1] 2D movement
  (if (not (Variables|Default|GetisDead))
    (Pawn|Input|AddMovementInput (Math|Vector|GetRightVector _returnvalue_2) (.x ActionValue) false)
    (Pawn|Input|AddMovementInput (Math|Vector|GetForwardVector _returnvalue_2) (.y ActionValue) false)))

(event Input|EnhancedActionEvents|EnhancedInputActionIA_Run
  (params (ActionValue :type Boolean) (ElapsedSeconds :type Float%20%28double-precision%29) (TriggeredSeconds :type Float%20%28double-precision%29) (InputAction :type Input%20Action%20Object%20Reference :default "/Game/Textures/Player/Input/IA_Run.IA_Run"))
  ;[1 1 1] 2D movement
  (:Triggered
    (Variables|Default|SetisRunning true :!label _label)
    (Variables|/Script/Engine.CharacterMovementComponent|SetMaxWalkSpeed (Variables|Character|GetCharacterMovement) (Variables|Default|GetrunSpeed)))
  (:Started
    (goto _label))
  (:Ongoing
    (goto _label))
  (:Canceled
    (Variables|Default|SetisRunning false :!label _label_2)
    (Variables|/Script/Engine.CharacterMovementComponent|SetMaxWalkSpeed (Variables|Character|GetCharacterMovement) (Variables|Default|GetwalkSpeed)))
  (:Completed
    (goto _label_2)))

(event Input|EnhancedActionEvents|EnhancedInputActionIA_Test
  (params (ActionValue :type Boolean) (ElapsedSeconds :type Float%20%28double-precision%29) (TriggeredSeconds :type Float%20%28double-precision%29) (InputAction :type Input%20Action%20Object%20Reference :default "/Game/Textures/Player/Input/IA_Test.IA_Test"))
  ;[1 1 1] Test
  (:Completed
    (CallFunction|DoThreePunchesAnimation)))

(event EventBeginPlay
  ;[1 1 1] Begin play
  ;;[1 1 1] Sprite flash setup
  (bind _returnvalue (Rendering|Material|CreateDynamicMaterialInstance (Variables|Default|GetSprite) 0 0 "None" :!class /Script/Engine.PrimitiveComponent))
  (Variables|Default|SetDynamicSpriteMaterial _returnvalue)
  ;;[1 1 1] HP system
  (Variables|Default|SetCurrentHP (Variables|Default|GetMaxHP))
  (Variables|Default|SetCurrentMP (Variables|Default|GetMaxMP))
  ;;[1 1 1] Input
  (bind _asplayer_controller (Utilities|Casting|CastToPlayerController (Pawn|GetController)))
  (Utilities|IsValid (PlayerController|LocalPlayerSubsystems|GetEnhancedInputLocalPlayerSubsystem _asplayer_controller)
    (:Is%20Valid
      (Input|AddMappingContext (PlayerController|LocalPlayerSubsystems|GetEnhancedInputLocalPlayerSubsystem _asplayer_controller) "/Game/Textures/Player/Input/IMC_Player.IMC_Player" 0 "(bIgnoreAllPressedKeysUntilRelease=True,bForceImmediately=False,bNotifyUserSettings=False)"))))

(event EventTick
  (params (DeltaSeconds :type Float%20%28single-precision%29))
  ;[1 1 1] Event tick
  (CallFunction|UpdateAnimations))

(fn ConstructionScript)

(fn GetHP
  (return (Math|Float|Truncate (Variables|Default|GetTargetHP))))

(fn GetMP
  (return (Math|Float|Truncate (Variables|Default|GetTargetMP))))

(fn GetHPPercent
  (return (/ (Variables|Default|GetCurrentHP) (Variables|Default|GetMaxHP))))

(fn GetMPPercent
  (return (/ (Variables|Default|GetCurrentMP) (Variables|Default|GetMaxMP))))

(fn RestoreHP
  (params (value :type Float%20%28double-precision%29))
  (CallFunction|PlayerDamaged (* value -1.0)))

(fn RestoreMP
  (params (value :type Float%20%28double-precision%29))
  (CallFunction|PlayerUseMP (* value -1.0)))

(fn RegenerateMP
  (CallFunction|RestoreMP (Variables|Default|GetMPRegen)))

(fn ToggleDefending
  (Variables|Default|SetisDefending (not (Variables|Default|GetisDefending))))

(fn ToggleinCombat
  (Variables|Default|SetisInCombat (not (Variables|Default|GetisInCombat))))